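; BP_Spawner_Parent is a base for capturable, upgradeable spawners tagged Player or Enemy by their WitchSpawner type.
; StartLoop runs a looping timer, while SelectAction draws an action from per-type DataTable probabilities and Level: spawn an AI unit, do nothing, or grant the player a resource.
; Upgrade spends player resources to raise Level.
; Capture counts entering units until a level-based threshold switches the spawner type, refreshes its tag and resets Level.
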(event Custom|SelectAction
  (bind _returnvalue (Utilities|GetDataTableRow (Variables|Default|GetDataTable) (Utilities|String|StringToName (Utilities|String|EnumtoString (Variables|Default|GetWitchSpawner))))
    (:then
      (bind _actionselect (CallFunction|SelectProba (.ProbaAction1 (Utilities|Struct|BreakST_BalancingBase _returnvalue)) (.ProbaAction2 (Utilities|Struct|BreakST_BalancingBase _returnvalue)) (.ProbaAction3 (Utilities|Struct|BreakST_BalancingBase _returnvalue)) (.ProbaAction4 (Utilities|Struct|BreakST_BalancingBase _returnvalue)) (.ProbaAction5 (Utilities|Struct|BreakST_BalancingBase _returnvalue)) (Variables|Default|GetLevel)))
      (Development|PrintString (Utilities|String|EnumtoString _actionselect))
      (switch Utilities|FlowControl|Switch|SwitchonE_ProbaAction _actionselect
        (:NewEnumerator0
          (CallFunction|Spawn))
        (:NewEnumerator1
          (CallFunction|Rien))
        (:NewEnumerator2
          (CallFunction|Ressource))))))

(event Custom|Start%20Loop
  (bind _returnvalue (Utilities|Time|SetTimerbyEvent (EventDispatchers|CreateEvent :!event Custom|SelectAction) (Variables|Default|GetTime%20for%20loop%20action) true))
  (Variables|Default|SetTimerHandle _returnvalue))

(event EventBeginPlay
  (Variables|Default|SetTags (Utilities|Array|MakeArray (select (Utilities|Enum|Equal(Enum) (Variables|Default|GetWitchSpawner) "NewEnumerator3") "Player" "Enemy"))))

(fn ConstructionScript)

(fn Spawn
  (bind _returnvalue (Game|SpawnActorfromClass "/Game/ABM_Content/ABM_Content/AI_Character/BP_AI_Parent.BP_AI_Parent_C" (Transformation|GetWorldTransform (Variables|Default|GetScene)) "Undefined" "MultiplyWithRoot" 0 (Variables|Default|GetLevel) (select (Utilities|Enum|Equal(Enum) (Variables|Default|GetWitchSpawner) "NewEnumerator0") "NewEnumerator1" "NewEnumerator0") 0))
  (AI|Components|Blackboard|SetValueasBool (AI|GetBlackboard _returnvalue) (LocalVariables|GetSpawn?) true))

(fn Rien)

(fn Ressource
  (bind _asbp_player_michel (Utilities|Casting|CastToBP_PlayerMichel (Game|GetPlayerCharacter 0)))
  (Variables|/Game/ABM_Content/ABM_Content/Player/BP_PlayerMichel.BP_PlayerMichel_C|SetRessourceCount _asbp_player_michel (+ (Variables|/Game/ABM_Content/ABM_Content/Player/BP_PlayerMichel.BP_PlayerMichel_C|GetRessourceCount _asbp_player_michel) 1)))

(fn Upgrade
  (bind _asbp_player_michel (Utilities|Casting|CastToBP_PlayerMichel (Game|GetPlayerCharacter 0)))
  (if (>= (Variables|/Game/ABM_Content/ABM_Content/Player/BP_PlayerMichel.BP_PlayerMichel_C|GetRessourceCount _asbp_player_michel) (Utilities|Array|Get(acopy) (Variables|Default|GetUpgradeCost) (- (Variables|Default|GetLevel) 1)))
    (Variables|/Game/ABM_Content/ABM_Content/Player/BP_PlayerMichel.BP_PlayerMichel_C|SetRessourceCount _asbp_player_michel (- (Variables|/Game/ABM_Content/ABM_Content/Player/BP_PlayerMichel.BP_PlayerMichel_C|GetRessourceCount _asbp_player_michel) (Utilities|Array|Get(acopy) (Variables|Default|GetUpgradeCost) (- (Variables|Default|GetLevel) 1))))
    (Variables|Default|SetLevel (+ (Variables|Default|GetLevel) 1))))

(fn Capture
  (bind _output_get (LocalVariables|SetUnit%20enter (+ (LocalVariables|GetUnit%20enter) 1)))
  (if (>= _output_get (Utilities|Array|Get(acopy) (Variables|Default|GetUnit%20for%20Conquet) (- (Variables|Default|GetLevel) 1)))
    (Variables|Default|SetWitchSpawner (select (Utilities|Enum|Equal(Enum) (Variables|Default|GetWitchSpawner) "NewEnumerator0") "NewEnumerator3" "NewEnumerator2"))
    (Utilities|Array|Clear (Variables|Actor|GetTags))
    (Variables|Default|SetTags (Utilities|Array|MakeArray (select (Utilities|Enum|Equal(Enum) (Variables|Default|GetWitchSpawner) "NewEnumerator0") "Player" "Enemy")))
    (Variables|Default|SetLevel 1)))