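; Base AI character for pawns split into Player and Enemy sides by the WitchPawn enum, which drives tag, random mesh and blue/red effect color.
; Player-side capsule hits on differing pawns halt both and write HitCharacter to the Blackboard.
; Percussion, string and wind track 3/4 skill events give Player-tagged pawns three-second timer-reverted buffs such as speed, level, instant kill or conversion flags.
; Death spawns a Niagara explosion and destroys the actor.
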(event OnComponentHit(CapsuleComponent)
  (params (HitComponent :type Primitive%20Component%20Object%20Reference) (OtherActor :type Actor%20Object%20Reference) (OtherComp :type Primitive%20Component%20Object%20Reference) (NormalImpulse :type Vector :default "0, 0, 0") (Hit :type Hit%20Result%20Structure%20%28by%20ref%29))
  (if (Utilities|Enum|Equal(Enum) (Variables|Default|GetWitchPawn) "NewEnumerator1")
    (bind _asbp_ai_parent (Utilities|Casting|CastToBP_AI_Parent OtherActor))
    (if (Utilities|Enum|NotEqual(Enum) (Variables|BP_AI_Parent_C|GetWitchPawn _asbp_ai_parent) (Variables|Default|GetWitchPawn))
      (Class|NavMovementInterface|StopActiveMovement (Variables|/Script/Engine.Character|GetCharacterMovement _asbp_ai_parent))
      (Class|NavMovementInterface|StopActiveMovement (Variables|Character|GetCharacterMovement))
      (AI|Components|Blackboard|SetValueasObject (AI|GetBlackboard 0) (Variables|Default|GetHitCharacter) _asbp_ai_parent))))

(event Custom|Competence%20Vent%20Track%204
  (if (== (Utilities|Array|Get(acopy) (Variables|Actor|GetTags)) "Player")
    (Variables|Default|SetMoveToAly true)
    (Utilities|Time|SetTimerbyEvent (delegate Custom|End%20Comp%203%20Track4) 3.0)))

(event Custom|Set%20Tag
  (bind _witchpawn (Variables|Default|GetWitchPawn))
  (bind _returnvalue (Utilities|Enum|Equal(Enum) _witchpawn "NewEnumerator1"))
  (Variables|Default|SetWitchCombat (select _returnvalue "NewEnumerator5" "NewEnumerator4"))
  (Variables|Default|SetTags (Utilities|Array|MakeArray (select _returnvalue "Player" "Enemy"))))

(event Custom|Competence%20Percution%20Track%203
  (if (== (Utilities|Array|Get(acopy) (Variables|Actor|GetTags)) "Player")
    (Variables|Default|SetInstantKill true)
    (Utilities|Time|SetTimerbyEvent (delegate Custom|End%20comp%201%20Track3) 3.0)))

(event Custom|Competenxce%20Corde%20Track%203
  (if (== (Utilities|Array|Get(acopy) (Variables|Actor|GetTags)) "Player")
    (Variables|Default|SetLevel (+ (Variables|Default|GetLevel) 1))
    (Utilities|Time|SetTimerbyEvent (delegate Custom|End%20Comp%202%20Track3) 3.0)))

(event Custom|Competence%20Vent%20Track%203
  (if (== (Utilities|Array|Get(acopy) (Variables|Actor|GetTags)) "Player")
    (Variables|Default|SetConvertDouble true)
    (Utilities|Time|SetTimerbyEvent (delegate Custom|End%20Comp%203%20Track3) 3.0)))

(event Custom|End%20comp%201%20Track3
  (Variables|Default|SetInstantKill false))

(event Custom|End%20Comp%202%20Track3
  (Variables|Default|SetLevel (- (Variables|Default|GetLevel) 1)))

(event Custom|End%20Comp%203%20Track3
  (Variables|Default|SetConvertDouble false))

(event Custom|Competence%20Percution%20Track%204
  (if (== (Utilities|Array|Get(acopy) (Variables|Actor|GetTags)) "Player")
    (Variables|/Script/Engine.CharacterMovementComponent|SetMaxWalkSpeed (Variables|Character|GetCharacterMovement) 5e+02)
    (Utilities|Time|SetTimerbyEvent (delegate Custom|End%20Comp%201%20Track4) 3.0)))

(event Custom|Competenxce%20Corde%20Track%204
  (if (== (Utilities|Array|Get(acopy) (Variables|Actor|GetTags)) "Player")
    (Variables|Default|SetPasIDLE true)
    (Utilities|Time|SetTimerbyEvent (delegate Custom|End%20Comp%202%20Track4) 3.0)))

(event Custom|End%20Comp%203%20Track4
  (Variables|Default|SetMoveToAly false))

(event Custom|End%20Comp%201%20Track4
  (Variables|/Script/Engine.CharacterMovementComponent|SetMaxWalkSpeed (Variables|Character|GetCharacterMovement) 3.5e+02))

(event Custom|End%20Comp%202%20Track4
  (Variables|Default|SetPasIDLE false))

(event EventBeginPlay
  (AI|Components|Blackboard|SetValueasBool (AI|GetBlackboard 0) (Variables|Default|GetSpawn?) true))

(fn ConstructionScript)

(fn Death
  (Niagara|SpawnSystematLocation "/Game/VFX/NS_DeadExplode.NS_DeadExplode" (Transformation|GetActorLocation))
  (Actor|DestroyActor))

(fn SetVisual
  (bind _witchpawn (Variables|Default|GetWitchPawn))
  (bind _truemesh (Variables|Default|GetTrueMesh))
  (bind _truemesh_2 (Variables|Default|GetTrueMesh))
  (if (Math|Boolean|ORBoolean (Utilities|Enum|Equal(Enum) _witchpawn "NewEnumerator1") (Utilities|Enum|Equal(Enum) _witchpawn "NewEnumerator3") (Utilities|Enum|Equal(Enum) _witchpawn "NewEnumerator5"))
    (switch int (Math|Random|RandomIntegerinRange 0 5)
      (:0
        (Variables|/Script/Engine.SkeletalMeshComponent|SetSkeletalMeshAsset _truemesh "/Game/DancingDudes/chara1/SK_gus1.SK_gus1")
        (Components|SkeletalMesh|SetAnimInstanceClass _truemesh "/Game/DancingDudes/chara1/BPA_gus1.BPA_gus1_C"))
      (:1
        (Variables|/Script/Engine.SkeletalMeshComponent|SetSkeletalMeshAsset _truemesh "/Game/DancingDudes/chara2/SK_gus2.SK_gus2")
        (Components|SkeletalMesh|SetAnimInstanceClass _truemesh "/Game/DancingDudes/chara2/BPA_gus2.BPA_gus2_C"))
      (:2
        (Variables|/Script/Engine.SkeletalMeshComponent|SetSkeletalMeshAsset _truemesh "/Game/DancingDudes/chara3/SK_Gus3.SK_Gus3")
        (Components|SkeletalMesh|SetAnimInstanceClass _truemesh "/Game/DancingDudes/chara3/ABP_retargGus3.ABP_retargGus3_C"))
      (:3
        (Variables|/Script/Engine.SkeletalMeshComponent|SetSkeletalMeshAsset _truemesh "/Game/DancingDudes/chara4/SK_gus4.SK_gus4")
        (Components|SkeletalMesh|SetAnimInstanceClass _truemesh "/Game/DancingDudes/chara4/BPA_gus4.BPA_gus4_C"))
      (:4
        (Variables|/Script/Engine.SkeletalMeshComponent|SetSkeletalMeshAsset _truemesh "/Game/DancingDudes/chara5/SK_gus5.SK_gus5")
        (Components|SkeletalMesh|SetAnimInstanceClass _truemesh "/Game/DancingDudes/chara5/BPA_chara5.BPA_chara5_C"))
      (:5
        (Variables|/Script/Engine.SkeletalMeshComponent|SetSkeletalMeshAsset _truemesh "/Game/DancingDudes/chara5/SK_gus5.SK_gus5")
        (Components|SkeletalMesh|SetAnimInstanceClass _truemesh "/Game/DancingDudes/chara6/BPA_chara6.BPA_chara6_C")))
    (Niagara|SetNiagaraVariable(LinearColor) (Variables|Default|GetNS_lileGus) "Color" (Class|KismetMathLibrary|LinearColorBlue))
    (else
      (switch int (Math|Random|RandomIntegerinRange 0 2)
        (:0
          (Variables|/Script/Engine.SkeletalMeshComponent|SetSkeletalMeshAsset _truemesh_2 "/Game/DancingDudes/Mechant1/SK_Mechant1.SK_Mechant1")
          (Components|SkeletalMesh|SetAnimInstanceClass _truemesh_2 "/Game/DancingDudes/Mechant1/ABP_MEchant1.ABP_MEchant1_C"))
        (:1
          (Variables|/Script/Engine.SkeletalMeshComponent|SetSkeletalMeshAsset _truemesh_2 "/Game/DancingDudes/Mechant2/SK_Mechant2.SK_Mechant2")
          (Components|SkeletalMesh|SetAnimInstanceClass _truemesh_2 "/Game/DancingDudes/Mechant2/ABP_MEchant2.ABP_MEchant2_C"))
        (:2
          (Variables|/Script/Engine.SkeletalMeshComponent|SetSkeletalMeshAsset _truemesh_2 "/Game/DancingDudes/Mechant3/SK_mechant3.SK_mechant3")
          (Components|SkeletalMesh|SetAnimInstanceClass _truemesh_2 "/Game/DancingDudes/Mechant3/ABP_Mechant3.ABP_Mechant3_C")))
      (Niagara|SetNiagaraVariable(LinearColor) (Variables|Default|GetNS_lileGus) "Color" (Class|KismetMathLibrary|LinearColorRed)))))